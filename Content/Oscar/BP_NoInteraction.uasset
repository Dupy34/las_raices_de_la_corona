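; Blueprint that blocks player interaction when play begins by disabling player controller input.
; BeginPlay also shows the mouse cursor, sets game-only input mode and prints a debug message.
; EnableInteract and DisableInteraction toggle CanInteract and controller input, then call UpdateInteractionState, which only prints the current state.
; An unconnected branch sketches a UI-only input mode with a test widget.
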(event EventBeginPlay
  (bind _returnvalue (Game|GetPlayerController 0))
  ;[0.15 0.15 0.15 0.5] Se asegura al 100% que no se interactua con nada
  (Input|DisableInput _returnvalue 0)
  (Variables|/Script/Engine.PlayerController|SetbShowMouseCursor _returnvalue true)
  (Input|SetInputModeGameOnly _returnvalue false)
  (Development|PrintString "NoInteractionActivated"))

(fn ConstructionScript)

(fn UpdateInteractionState
  ;[0.15 0.15 0.15 0.5] Cosas para la UI
  (if (Variables|Default|GetCanInteract)
    (Development|PrintString "puede decidir" true true "(R=0.000000,G=1.000000,B=0.198892,A=1.000000)")
    (else
      (Development|PrintString "no puede decidir" true true "(R=1.000000,G=0.000000,B=0.000000,A=1.000000)"))))

(fn EnableInteract
  (bind _returnvalue (Game|GetPlayerController 0))
  ;[0.15 0.15 0.15 0.5] cosas para la UI
  (Variables|Default|SetCanInteract true)
  (Input|EnableInput _returnvalue _returnvalue)
  (CallFunction|UpdateInteractionState))

(fn DisableInteraction
  (bind _returnvalue (Game|GetPlayerController 0))
  ;[0.15 0.15 0.15 0.5] cosa para la UI
  (Variables|Default|SetCanInteract false)
  (Input|DisableInput _returnvalue _returnvalue)
  (CallFunction|UpdateInteractionState))